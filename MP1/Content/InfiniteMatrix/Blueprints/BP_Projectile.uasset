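; BP_Projectile is a projectile that scores points by destroying enemies on contact.
; When its collision component overlaps a BP_Enermy, it prints a hit message, adds one to the player pawn's ScoreGet, then destroys the enemy and itself.
; Hitting a BP_HealthPack destroys only the projectile.
; Tick accumulates delta time so the projectile self-destructs after twenty seconds.
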(event `self.ReceiveTick`
  (params (DeltaSeconds :type "Float (single-precision)"))
  (bind _output_get (set `self.Delta` (+ DeltaSeconds (`self.Delta`))))
  (if (>= _output_get 20.0)
    (`self.K2_DestroyActor`)))

(event `self.Projectile.OnComponentBeginOverlap`
  (params (OverlappedComponent :type "PrimitiveComponent Object Reference") (OtherActor :type "Actor Object Reference") (OtherComp :type "PrimitiveComponent Object Reference") (OtherBodyIndex :type Integer) (bFromSweep :type Boolean) (SweepResult :type "HitResult Structure (by ref)"))
  (bind _asbp_enermy (cast `/Game/InfiniteMatrix/Blueprints/BP_Enermy` OtherActor)
    (:`then`
      (bind _asbp_player (cast `/Game/InfiniteMatrix/Blueprints/BP_Player` (`GameplayStatics.GetPlayerPawn` 0)))
      (`KismetSystemLibrary.PrintString` "Hit +")
      (set `/Game/InfiniteMatrix/Blueprints/BP_Player.Score_Get` (+ (`/Game/InfiniteMatrix/Blueprints/BP_Player.Score_Get` _asbp_player) 1) _asbp_player)
      (`self.K2_DestroyActor` _asbp_enermy)
      (`self.K2_DestroyActor` self))
    (:`CastFailed`
      (cast `/Game/InfiniteMatrix/Blueprints/BP_HealthPack` OtherActor)
      (`self.K2_DestroyActor` self))))

(fn `UserConstructionScript`)