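; BP_HealthPack is a health pickup that restores a small fixed amount of HP to the player.
; When its Healthcon component overlaps a BP_Player, it adds the heal to HPRecent, caps it at HPMax and destroys itself.
; Tick accumulates delta time and destroys an uncollected pack after 20 seconds.
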(event `self.ReceiveTick`
  (params (DeltaSeconds :type "Float (single-precision)"))
  (bind _output_get (set `self.Delta` (+ DeltaSeconds (`self.Delta`))))
  (if (>= _output_get 20.0)
    (`self.K2_DestroyActor`)))

(event `self.Healthcon.OnComponentBeginOverlap`
  (params (OverlappedComponent :type "PrimitiveComponent Object Reference") (OtherActor :type "Actor Object Reference") (OtherComp :type "PrimitiveComponent Object Reference") (OtherBodyIndex :type Integer) (bFromSweep :type Boolean) (SweepResult :type "HitResult Structure (by ref)"))
  (bind _asbp_player (cast `/Game/InfiniteMatrix/Blueprints/BP_Player` OtherActor))
  (bind _returnvalue (+ (`/Game/InfiniteMatrix/Blueprints/BP_Player.HP_recent` _asbp_player) 10))
  (bind _hp_max (`/Game/InfiniteMatrix/Blueprints/BP_Player.HP_max` _asbp_player))
  (if (>= _returnvalue _hp_max)
    (set `/Game/InfiniteMatrix/Blueprints/BP_Player.HP_recent` _hp_max _asbp_player)
    (else
      (set `/Game/InfiniteMatrix/Blueprints/BP_Player.HP_recent` _returnvalue _asbp_player)))
  (`self.K2_DestroyActor`))

(fn `UserConstructionScript`)